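; Gameplay game mode that tracks player controllers, spawns players as their chosen character and handles logout.
; RespawnPlayers destroys the controller's current pawn, spawns the supplied character class at a random PlayerStart and possesses it.
; Controllers arriving through OnSwapPlayerControllers are added to a list.
; On logout, a GamePlay_PC is passed to GameInfoInstance's DestroySessionCaller to tear down the session.
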(event Custom|Respawn%20Players
  (params (Player%20controller :type Player%20Controller%20Object%20Reference) (Player%20Character :type Character%20Class%20Reference))
  (bind _returnvalue (Pawn|GetControlledPawn Player%20controller))
  ;[1 1 1] Spawn the player with their Selected character From the game play PC
  (bind _outactors (Actor|GetAllActorsOfClass "/Script/Engine.PlayerStart"))
  (Variables|Default|SetSpawn%20Points _outactors)
  (Utilities|IsValid _returnvalue
    (:Is%20Valid
      (Actor|DestroyActor _returnvalue))
    (:Is%20Not%20Valid
      _))
  (bind _returnvalue_2 (Game|SpawnActorfromClass Player%20Character (Transformation|GetActorTransform (Utilities|Array|Get(acopy) (Variables|Default|GetSpawn%20Points) (Math|Random|RandomIntegerinRange 0 (Utilities|Array|LastIndex (Variables|Default|GetSpawn%20Points))))) "Undefined" 0 0))
  (Pawn|Possess Player%20controller _returnvalue_2))

(event EventOnSwapPlayerControllers
  (params (OldPC :type Player%20Controller%20Object%20Reference) (NewPC :type Player%20Controller%20Object%20Reference))
  ;[1 1 1] Keep Track on all player controllers
  (Utilities|Array|Add (Variables|Default|GetAll%20PlayerControllers) NewPC))

(event EventOnLogout
  (params (ExitingController :type Controller%20Object%20Reference))
  ;[1 1 1] Event On logout- Destroy Session Caller in Game info instance
  (bind _asgame_play_pc (Utilities|Casting|CastToGamePlay_PC ExitingController))
  (Default|DestroySessionCaller (.AsGame%20Info%20Instance (Utilities|Casting|CastToGameInfoInstance (Game|GetGameInstance))) _asgame_play_pc))

(fn ConstructionScript)